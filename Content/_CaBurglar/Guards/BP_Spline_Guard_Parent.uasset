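; Parent guard Blueprint for a stealth game that patrols a spline, hunts the player and restarts the level on capture.
; A timeline samples spline points for AIMoveTo, while AI perception feeds a looping timer that raises or decays suspicion.
; Suspicion thresholds and lost sight switch between Patrol, Search at the last known location with a look-around, and Chase, recoloring the vision cone light.
; Capture disables input, fades the camera and reloads the level.
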(event `ConeColorShift`
  ; ConeColorShift
  (switch `/Game/_CaBurglar/Guards/Enum_GuardState` (`self.GuardState`)
    (:`NewEnumerator0`
      (`LightComponent.SetLightColor` (`self.VisionCone`) (struct :`R` 0.212231 :`G` 0.296138 :`B` 0.879623 :`A` 1.0) true))
    (:`NewEnumerator1`
      (`LightComponent.SetLightColor` (`self.VisionCone`) (struct :`R` 1.0 :`G` 1.0 :`A` 1.0) true)
      (`GameplayStatics.PlaySound2D` "/Game/_CaBurglar/Guards/SFX/SC_Guard.SC_Guard" 1.0 1.0 0.0 null null))
    (:`NewEnumerator2`
      (`LightComponent.SetLightColor` (`self.VisionCone`) (struct :`R` 1.0 :`A` 1.0) true)
      (`TimelineComponent.Stop` (`self.TL_Patrol`))
      (`TimelineComponent.Stop` (`self.TL_LookAround`))
      (`/Engine/EditorBlueprintResources/StandardMacros.DoOnce` false
        (:`Completed`
          (`GameplayStatics.PlaySound2D` "/Game/_CaBurglar/Guards/SFX/Caught.Caught" 1.0 1.0 0.0 null null))))))

(event `self.ReceiveBeginPlay`
  ; BeginPlay/Patrol
  (`self.Patrol`))

(event `Patrol`
  (bind _spline (`/Game/_CaBurglar/Guards/BP_Spline_Parent.Spline` (`self.SplineReference`)))
  ; BeginPlay/Patrol
  (`self.ConeColorShift`)
  (if (`|EnumEquality` (`self.GuardState`) "NewEnumerator0")
    (`TimelineComponent.SetPlayRate` (`self.TL_Patrol`) (/ 1.0 (`self.TimeToComplete`)))
    (bind (_direction _movetrack) (`Timeline|TL_Patrol` :!label _label)
      (:`Update`
        (`|AIMoveTo` self (`SplineComponent.GetLocationAtDistanceAlongSpline` _spline (`KismetMathLibrary.Lerp` 0.0 (`SplineComponent.GetSplineLength` _spline) _movetrack) "World") null 0.1
          (:`then`
            (`KismetSystemLibrary.Delay` (`self.TimeToComplete`))
            (`self.Patrol`)))))
    (else
      (goto _label :!via `Stop`))))

(event `self.AIPerception.OnTargetPerceptionUpdated`
  (params (Actor :type "Actor Object Reference") (Stimulus :type "AIStimulus Structure"))
  ; AIPerception
  (bind _asbp_third_person_character (cast `/Game/ThirdPerson/Blueprints/BP_ThirdPersonCharacter` Actor))
  (if Stimulus_bSuccessfullySensed
    (set `self.CanSeePlayer` true)
    (if (`KismetSystemLibrary.K2_IsTimerActiveHandle` (`self.SuspicionHandle`))
      (if (<= (`self.Suspicion`) 0.0)
        (`KismetSystemLibrary.K2_ClearAndInvalidateTimerHandle` (`self.SuspicionHandle`)))
      (else
        (bind _returnvalue (`KismetSystemLibrary.K2_SetTimer` null "SuspicionTick" 0.2 true true))
        (set `self.SuspicionHandle` _returnvalue)))
    (else
      (set `self.CanSeePlayer` false)
      (`self.Search`))))

(event `Chase`
  ; AIPerception
  (`TimelineComponent.Stop` (`self.TL_Patrol`))
  (set `self.IsChasing` true)
  (set `self.GuardState` "NewEnumerator2")
  (`self.ConeColorShift`)
  (`|AIMoveTo` self (0.0 0.0 0.0) (stale `self.AIPerception.OnTargetPerceptionUpdated` _asbp_third_person_character) 5.0 true
    (:`OnSuccess`
      (`MovementComponent.StopMovementImmediately` (`self.CharacterMovement`))
      (`self.Caught`))))

(event `SuspicionTick`
  ; SuspicionTick
  (if (`self.CanSeePlayer`)
    (set `self.LastKnownLocation` (`self.K2_GetActorLocation` (`GameplayStatics.GetPlayerCharacter` 0)))
    (set `self.Suspicion` (`KismetMathLibrary.FClamp` (+ (`self.Suspicion`) (* (`self.SuspicionIncreaseRate`) 0.2)) 0.0 50.0))
    (if (and (>= (`self.Suspicion`) (`self.ChaseThreshold`)) (`|EnumInequality` (`self.GuardState`) "NewEnumerator2"))
      (set `self.GuardState` "NewEnumerator2")
      (`MovementComponent.StopMovementImmediately` (`self.CharacterMovement`))
      (`self.ConeColorShift`)
      (`self.Chase`))
    (else
      (set `self.Suspicion` (`KismetMathLibrary.FClamp` (- (`self.Suspicion`) (* (`self.SuspicionDecayRate`) 0.2)) 0.0 50.0))
      (if (and (<= (`self.Suspicion`) (`self.LoseChaseThreshold`)) (`|EnumEquality` (`self.GuardState`) "NewEnumerator2"))
        (set `self.GuardState` "NewEnumerator1")
        (`MovementComponent.StopMovementImmediately` (`self.CharacterMovement`))
        (`TimelineComponent.Stop` (`self.TL_Patrol`))
        (`self.ConeColorShift`)
        (`self.Search`)))))

(event `Search`
  ; Search
  (set `self.GuardState` "NewEnumerator1")
  (`self.ConeColorShift`)
  (`MovementComponent.StopMovementImmediately` (`self.CharacterMovement`))
  (`TimelineComponent.Stop` (`self.TL_Patrol`))
  (`|AIMoveTo` self (`self.LastKnownLocation`) null
    (:`OnSuccess`
      (`MovementComponent.StopMovementImmediately` (`self.CharacterMovement`))
      (`self.LookAround`))
    (:`OnFail`
      (`self.LookAround`))))

(event `LookAround`
  (bind (_guardrotation_roll _guardrotation_pitch _guardrotation_yaw) (`KismetMathLibrary.BreakRotator` (`self.GuardRotation`)))
  ; LookAround
  (if (`|EnumEquality` (`self.GuardState`) "NewEnumerator2")
    (bind (_direction _yawoffset) (`Timeline|TL_LookAround` :!via `Stop` :!label _label_2)
      (:`Update`
        (`self.K2_SetActorRotation` self (`KismetMathLibrary.MakeRotator` 0.0 0.0 (+ _guardrotation_yaw _yawoffset)) false))
      (:`Finished`
        (`KismetSystemLibrary.Delay` 2.0)
        (set `self.GuardState` "NewEnumerator0")
        (`self.Patrol`)
        (`KismetSystemLibrary.K2_ClearTimer` self "SuspicionTick")))
    (else
      (set `self.GuardRotation` (`self.K2_GetActorRotation` self))
      (goto _label_2 :!via `PlayFromStart`))))

(event `self.CapsuleComponent.OnComponentHit`
  (params (HitComponent :type "PrimitiveComponent Object Reference") (OtherActor :type "Actor Object Reference") (OtherComp :type "PrimitiveComponent Object Reference") (NormalImpulse :type "Vector Structure") (Hit :type "HitResult Structure (by ref)"))
  ; Caught
  (cast `/Game/ThirdPerson/Blueprints/BP_ThirdPersonCharacter` OtherActor)
  (if (`self.CanSeePlayer`)
    (`/Engine/EditorBlueprintResources/StandardMacros.DoOnce` false
      (:`Completed`
        (`MovementComponent.StopMovementImmediately` (`self.CharacterMovement`))
        (`TimelineComponent.Stop` (`self.TL_Patrol`))
        (`TimelineComponent.Stop` (`self.TL_LookAround`))
        (`SkeletalMeshComponent.PlayAnimation` (`self.Mesh`) "/Game/_CaBurglar/Guards/Animations/Run_To_Stop.Run_To_Stop" false)
        (`self.Caught`)))))

(event `Caught`
  (bind _returnvalue (`GameplayStatics.GetPlayerCharacter` 0))
  ; Caught
  (`/Engine/EditorBlueprintResources/StandardMacros.DoOnce` false
    (:`Completed`
      (`SkeletalMeshComponent.PlayAnimation` (`Character.Mesh` _returnvalue) "/Game/StylizedCreaturesBundle/Animations/Cat/A_Cat_Idle01.A_Cat_Idle01" false)
      (`self.DisableInput` _returnvalue null)
      (`PlayerCameraManager.StartCameraFade` (`GameplayStatics.GetPlayerCameraManager` 0) 0.0 1.0 3.5 (struct :`A` 1.0) true false)
      (`GameplayStatics.PlaySound2D` "/Game/_CaBurglar/Cat/SFX/SC_Caught.SC_Caught" 1.0 1.0 0.0 null null)
      (`KismetSystemLibrary.Delay` 3.5)
      (bind _returnvalue_2 (`GameplayStatics.GetCurrentLevelName` true))
      (`GameplayStatics.OpenLevel` (`KismetStringLibrary.Conv_StringToName` _returnvalue_2)))))

(event `ResetTrack`)

(fn `UserConstructionScript`)