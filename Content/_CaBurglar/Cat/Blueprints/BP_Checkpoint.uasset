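; Checkpoint actor for the third-person game, built around a box trigger and a scene component.
; The Construction Script sizes the box from per-instance extent variables.
; Its box overlap event is empty, so the checkpoint currently saves nothing.
; Disconnected logic would cast to the player character and game mode, then store the scene component's world location as the game mode's PlayerLocation.
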(event `self.Box.OnComponentBeginOverlap`
  (params (OverlappedComponent :type "PrimitiveComponent Object Reference") (OtherActor :type "Actor Object Reference") (OtherComp :type "PrimitiveComponent Object Reference") (OtherBodyIndex :type Integer) (bFromSweep :type Boolean) (SweepResult :type "HitResult Structure (by ref)")))

(fn `UserConstructionScript`
  (`BoxComponent.SetBoxExtent` (`self.Box`) (`KismetMathLibrary.MakeVector` (`self.In Box Extent X`) (`self.In Box Extent Y`) (`self.In Box Extent Z`)) true))