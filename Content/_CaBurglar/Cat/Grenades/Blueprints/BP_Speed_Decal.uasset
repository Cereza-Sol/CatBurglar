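; Temporary speed-boost zone, filed with the grenades, that makes the player character walk faster.
; Box overlap by the player pawn raises the character's MaxWalkSpeed, and leaving restores a fixed normal speed after a delay.
; The actor destroys itself about five seconds after BeginPlay, so the delayed reset only completes if the player exits almost immediately after spawn.
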(event `self.ReceiveBeginPlay`
  (`KismetSystemLibrary.Delay` 5.1)
  (`self.K2_DestroyActor`))

(event `self.Box.OnComponentBeginOverlap`
  (params (OverlappedComponent :type "PrimitiveComponent Object Reference") (OtherActor :type "Actor Object Reference") (OtherComp :type "PrimitiveComponent Object Reference") (OtherBodyIndex :type Integer) (bFromSweep :type Boolean) (SweepResult :type "HitResult Structure (by ref)"))
  (bind _returnvalue (`GameplayStatics.GetPlayerPawn` 0))
  (if (== OtherActor _returnvalue)
    (`KismetSystemLibrary.PrintString` "Speed Activated")
    (bind _asbp_third_person_character (cast `/Game/ThirdPerson/Blueprints/BP_ThirdPersonCharacter` _returnvalue))
    (set `CharacterMovementComponent.MaxWalkSpeed` 800.0 (`Character.CharacterMovement` _asbp_third_person_character))))

(event `self.Box.OnComponentEndOverlap`
  (params (OverlappedComponent :type "PrimitiveComponent Object Reference") (OtherActor :type "Actor Object Reference") (OtherComp :type "PrimitiveComponent Object Reference") (OtherBodyIndex :type Integer))
  (bind _returnvalue (`GameplayStatics.GetPlayerPawn` 0))
  (if (== OtherActor _returnvalue)
    (`KismetSystemLibrary.Delay` 5.0)
    (`KismetSystemLibrary.PrintString` "Speed DIsabled")
    (bind _asbp_third_person_character (cast `/Game/ThirdPerson/Blueprints/BP_ThirdPersonCharacter` _returnvalue))
    (set `CharacterMovementComponent.MaxWalkSpeed` 600.0 (`Character.CharacterMovement` _asbp_third_person_character))))

(fn `UserConstructionScript`)