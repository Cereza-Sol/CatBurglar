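; BP_Shadow_Decal is a temporary shadow zone, apparently from a grenade, that hides the player character from AI sight.
; Box overlap unregisters a BP_ThirdPersonCharacter's stimuli source from the sight sense and clears CanBeSeen, and end overlap restores both, each printing a debug message.
; The actor destroys itself after a short fixed delay following BeginPlay.
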(event `self.ReceiveBeginPlay`
  (`KismetSystemLibrary.Delay` 6.0)
  (`self.K2_DestroyActor`))

(event `self.Box.OnComponentBeginOverlap`
  (params (OverlappedComponent :type "PrimitiveComponent Object Reference") (OtherActor :type "Actor Object Reference") (OtherComp :type "PrimitiveComponent Object Reference") (OtherBodyIndex :type Integer) (bFromSweep :type Boolean) (SweepResult :type "HitResult Structure (by ref)"))
  (bind _asbp_third_person_character (cast `/Game/ThirdPerson/Blueprints/BP_ThirdPersonCharacter` OtherActor))
  (`AIPerceptionStimuliSourceComponent.UnregisterFromSense` (`/Game/ThirdPerson/Blueprints/BP_ThirdPersonCharacter.AIPerceptionStimuliSource` _asbp_third_person_character) "/Script/AIModule.AISense_Sight")
  (set `/Game/ThirdPerson/Blueprints/BP_ThirdPersonCharacter.CanBeSeen` false _asbp_third_person_character)
  (`KismetSystemLibrary.PrintString` "Cannot Be Seen"))

(event `self.Box.OnComponentEndOverlap`
  (params (OverlappedComponent :type "PrimitiveComponent Object Reference") (OtherActor :type "Actor Object Reference") (OtherComp :type "PrimitiveComponent Object Reference") (OtherBodyIndex :type Integer))
  (bind _asbp_third_person_character (cast `/Game/ThirdPerson/Blueprints/BP_ThirdPersonCharacter` OtherActor))
  (`AIPerceptionStimuliSourceComponent.RegisterForSense` (`/Game/ThirdPerson/Blueprints/BP_ThirdPersonCharacter.AIPerceptionStimuliSource` _asbp_third_person_character) "/Script/AIModule.AISense_Sight")
  (set `/Game/ThirdPerson/Blueprints/BP_ThirdPersonCharacter.CanBeSeen` true _asbp_third_person_character)
  (`KismetSystemLibrary.PrintString` "Can Be Seen"))

(fn `UserConstructionScript`)