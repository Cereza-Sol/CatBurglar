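; BP_Shadowball_Grenade is a short-lived physics grenade that casts a shadow decal onto the surface below it.
; On spawn, a timeline drives its uniform scale, and the actor destroys itself after a fixed delay.
; Shortly after spawn, a debug-drawn downward trace places BP_Shadow_Decal at the hit, aligned to the surface normal and the sphere's velocity projected onto that surface.
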(event `self.ReceiveBeginPlay`
  (`self.Scale`)
  (`self.CastShadow`)
  (`KismetSystemLibrary.Delay` 2.0)
  (`self.K2_DestroyActor`))

(event `Scale`
  (bind (_direction _scaleamount) (`Timeline|Shrink`)
    (:`Update`
      (`self.SetActorScale3D` (`KismetMathLibrary.MakeVector` _scaleamount _scaleamount _scaleamount)))))

(event `CastShadow`
  (`KismetSystemLibrary.Delay` 0.5)
  (bind _outhit (`KismetSystemLibrary.LineTraceSingle` :`Start` (`self.K2_GetActorLocation`) :`End` (+ (`self.K2_GetActorLocation` self) (`KismetMathLibrary.MakeVector` 0.0 0.0 -1000.0)) :`TraceChannel` "TraceTypeQuery1" :`DrawDebugType` "ForDuration" :`DrawTime` 1.0))
  (bind _returnvalue (`PrimitiveComponent.GetPhysicsLinearVelocity` (`self.Sphere`) "None"))
  (`|SpawnActorFromClass` "/Game/_CaBurglar/Cat/Grenades/Blueprints/BP_Shadow_Decal.BP_Shadow_Decal_C" (`KismetMathLibrary.MakeTransform` (`.Location` (`GameplayStatics.BreakHitResult` _outhit)) (`KismetMathLibrary.MakeRotFromZY` (`.Normal` (`GameplayStatics.BreakHitResult` _outhit)) (`KismetMathLibrary.Normal` (`KismetMathLibrary.ProjectVectorOnToPlane` _returnvalue (`.ImpactNormal` (`GameplayStatics.BreakHitResult` _outhit)))))) "Undefined" "MultiplyWithRoot" null null))

(fn `UserConstructionScript`)