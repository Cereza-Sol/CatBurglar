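; BP_Speed_Grenade is a grenade actor that places a BP_Speed_Decal on the surface beneath it.
; On BeginPlay it runs CastSpeed, which traces straight down on the Visibility channel and spawns the decal at the hit point, oriented to the surface normal.
; The trace draws debug lines and its hit result goes unchecked before spawning.
; The grenade destroys itself after a short delay.
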(event `self.ReceiveBeginPlay`
  (`self.CastSpeed`)
  (`KismetSystemLibrary.Delay` 3.0)
  (`self.K2_DestroyActor`))

(event `CastSpeed`
  (bind _outhit (`KismetSystemLibrary.LineTraceSingle` :`Start` (`self.K2_GetActorLocation`) :`End` (+ (`self.K2_GetActorLocation` self) (`KismetMathLibrary.MakeVector` 0.0 0.0 -1000.0)) :`TraceChannel` "TraceTypeQuery1" :`DrawDebugType` "ForDuration" :`DrawTime` 1.0))
  (`|SpawnActorFromClass` "/Game/_CaBurglar/Cat/Grenades/Blueprints/BP_Speed_Decal.BP_Speed_Decal_C" (`KismetMathLibrary.MakeTransform` (`.Location` (`GameplayStatics.BreakHitResult` _outhit)) (`KismetMathLibrary.MakeRotFromZ` (`.Normal` (`GameplayStatics.BreakHitResult` _outhit)))) "Undefined" "MultiplyWithRoot" null null))

(fn `UserConstructionScript`)