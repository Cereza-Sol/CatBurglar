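; BP_Spotlight_Master is a configurable spotlight fixture that pairs a SpotLight with a mesh whose emissive material matches the light.
; The Construction Script applies variables for offset, rotation, intensity, cone angles, attenuation radius and color to the SpotLight.
; It then creates a dynamic instance of M_Emmisive_Master on mesh material slot 1, driving its color and emissive intensity from the same light color and intensity.
; The event graph has no active logic.
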(fn `UserConstructionScript`
  (bind _spotlight (`self.SpotLight`))
  (`SceneComponent.K2_SetRelativeLocationAndRotation` _spotlight (`self.LightOffset`) (`self.LightRotation`) false false)
  (`LightComponent.SetIntensity` _spotlight (`self.LightIntensity`))
  (`SpotLightComponent.SetInnerConeAngle` _spotlight (`self.Innercone`))
  (`SpotLightComponent.SetOuterConeAngle` _spotlight (`self.OuterCone`))
  (`LocalLightComponent.SetAttenuationRadius` _spotlight (`self.AttenuationRadius`))
  (`LightComponent.SetLightColor` _spotlight (`self.LightColor`) true)
  (bind _returnvalue (`PrimitiveComponent.CreateDynamicMaterialInstance` (`self.Mesh`) 1 "/Game/DavidFolder/Materials/M_Emmisive_Master.M_Emmisive_Master" "None"))
  (bind _output_get (set `self.EmmisiveMaterial` _returnvalue))
  (`MaterialInstanceDynamic.SetVectorParameterValue` _output_get "Color" (`self.LightColor`))
  (`MaterialInstanceDynamic.SetScalarParameterValue` _output_get "EmissiveIntensity" (`self.LightIntensity`)))