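; Master loot pickup that spins in place and increments the player character's LootCollected count when collected.
; A looping timeline drives the mesh's yaw from BeginPlay.
; Overlap of the sphere by BP_ThirdPersonCharacter destroys the actor, plays a 2D sound and updates the count on player 0.
; The construction script applies configurable mesh and spotlight settings, reusing light color and intensity in a dynamic emissive material.
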(event `self.ReceiveBeginPlay`
  (`self.RotateBox`))

(event `self.Sphere.OnComponentBeginOverlap`
  (params (OverlappedComponent :type "PrimitiveComponent Object Reference") (OtherActor :type "Actor Object Reference") (OtherComp :type "PrimitiveComponent Object Reference") (OtherBodyIndex :type Integer) (bFromSweep :type Boolean) (SweepResult :type "HitResult Structure (by ref)"))
  (cast `/Game/ThirdPerson/Blueprints/BP_ThirdPersonCharacter` OtherActor)
  (`self.K2_DestroyActor`)
  (`GameplayStatics.PlaySound2D` "/Game/_CaBurglar/Cat/SFX/TreatBox_001.TreatBox_001" 1.0 1.0 0.0 null null)
  (bind _asbp_third_person_character (cast `/Game/ThirdPerson/Blueprints/BP_ThirdPersonCharacter` (`GameplayStatics.GetPlayerCharacter` 0)))
  (bind _result (`/Engine/EditorBlueprintResources/StandardMacros.IncrementInt` (`/Game/ThirdPerson/Blueprints/BP_ThirdPersonCharacter.LootCollected` _asbp_third_person_character))
    (:`  `
      (set `self.LootCollected` _result))))

(event `RotateBox`
  (bind (_boxrotation_roll _boxrotation_pitch _boxrotation_yaw) (`KismetMathLibrary.BreakRotator` (`self.BoxRotation`)))
  (bind (_direction _yawoffset) (`Timeline|Rotating` :!via `PlayFromStart`)
    (:`Update`
      (`SceneComponent.K2_SetWorldRotation` (`self.LootMesh`) (`KismetMathLibrary.MakeRotator` 0.0 0.0 (+ _boxrotation_yaw _yawoffset)) false false))
    (:`Finished`
      (`self.RotateBox`))))

(fn `UserConstructionScript`
  (bind _spotlight (`self.SpotLight`))
  (`StaticMeshComponent.SetStaticMesh` (`self.LootMesh`) (`self.NewLootMesh`))
  (`SceneComponent.K2_SetRelativeLocationAndRotation` _spotlight (`self.Light Location`) (`self.Light Rotation`) false false)
  (`LightComponent.SetIntensity` _spotlight (`self.LightIntensity`))
  (`SpotLightComponent.SetInnerConeAngle` _spotlight (`self.InnerConeAngle`))
  (`SpotLightComponent.SetOuterConeAngle` _spotlight (`self.OuterConeAngle`))
  (`LocalLightComponent.SetAttenuationRadius` _spotlight (`self.AttenuationRadius`))
  (`LightComponent.SetLightColor` _spotlight (`self.LightColor`) true)
  (bind _returnvalue (`PrimitiveComponent.CreateDynamicMaterialInstance` (`self.LootMesh`) 1 "/Game/DavidFolder/Materials/M_Emmisive_Master.M_Emmisive_Master" "None"))
  (bind _output_get (set `self.EmmisiveMaterial` _returnvalue))
  (`MaterialInstanceDynamic.SetVectorParameterValue` _output_get "Color" (`self.LightColor`))
  (`MaterialInstanceDynamic.SetScalarParameterValue` _output_get "EmissiveIntensity" (`self.LightIntensity`)))