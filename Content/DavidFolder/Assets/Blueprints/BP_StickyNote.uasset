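; BP_StickyNote is a readable note that shows its text on screen while the player is near it.
; When the player character enters its Box, it creates a WB_Notes widget with its Text variable, stores the reference and adds it to the viewport.
; Leaving the Box removes that widget, and each transition plays its own 2D note sound.
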(event `self.Box.OnComponentBeginOverlap`
  (params (OverlappedComponent :type "PrimitiveComponent Object Reference") (OtherActor :type "Actor Object Reference") (OtherComp :type "PrimitiveComponent Object Reference") (OtherBodyIndex :type Integer) (bFromSweep :type Boolean) (SweepResult :type "HitResult Structure (by ref)"))
  (if (== OtherActor (`GameplayStatics.GetPlayerCharacter` 0))
    (bind _returnvalue (`|CreateWidget` "/Game/_CaBurglar/Widgets/WB_Notes.WB_Notes_C" null (`self.Text`)))
    (bind _output_get (set `self.NoteWidgetRef` _returnvalue))
    (`UserWidget.AddToViewport` _output_get 0)
    (`GameplayStatics.PlaySound2D` "/Game/_CaBurglar/Cat/SFX/Note_03.Note_03" 1.0 1.0 0.0 null null)))

(event `self.Box.OnComponentEndOverlap`
  (params (OverlappedComponent :type "PrimitiveComponent Object Reference") (OtherActor :type "Actor Object Reference") (OtherComp :type "PrimitiveComponent Object Reference") (OtherBodyIndex :type Integer))
  (if (== OtherActor (`GameplayStatics.GetPlayerCharacter` 0))
    (`Widget.RemoveFromParent` (`self.NoteWidgetRef`))
    (`GameplayStatics.PlaySound2D` "/Game/_CaBurglar/Cat/SFX/Note_02.Note_02" 1.0 1.0 0.0 null null)))

(fn `UserConstructionScript`)